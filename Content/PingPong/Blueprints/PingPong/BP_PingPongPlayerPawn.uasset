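; Player pawn for the PingPong game that handles debug-style pause and score input.
; Q toggles game pause through a FlipFlop.
; Tab calls the Score event, which casts the GameState to PingPongGameStateBase and prints the blue and green player scores and ball hit count to screen.
; BeginPlay, Tick and the construction script are empty.
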(event `Key|Q`
  (params (Key :type "Key Structure"))
  (:`Pressed`
    (`/Engine/EditorBlueprintResources/StandardMacros.FlipFlop`
      (:`A`
        (`GameplayStatics.SetGamePaused` true))
      (:`B`
        (`GameplayStatics.SetGamePaused` false)))))

(event `self.ReceiveBeginPlay`)

(event `self.ReceiveTick`
  (params (DeltaSeconds :type "Float (single-precision)")))

(event `Key|Tab`
  (params (Key :type "Key Structure"))
  (:`Pressed`
    (`self.Score`)))

(event `Score`
  ;[1 1 1] Score
  (bind _asping_pong_game_state_base (cast `PingPongGameStateBase` (`GameplayStatics.GetGameState`))
    (:`then`
      (bind _returnvalue (`PingPongGameStateBase.GetScoreBluePlayer` _asping_pong_game_state_base))
      (bind _returnvalue_2 (`PingPongGameStateBase.GetScoreGreenPlayer` _asping_pong_game_state_base))
      (bind _returnvalue_3 (`PingPongGameStateBase.GetBallHits` _asping_pong_game_state_base))
      (`KismetSystemLibrary.PrintString` (`KismetStringLibrary.Concat_StrStr` (`KismetStringLibrary.Conv_IntToString` _returnvalue) "     " (`KismetStringLibrary.Conv_IntToString` _returnvalue_2) "  hits:" (`KismetStringLibrary.Conv_IntToString` _returnvalue_3))))
    (:`CastFailed`
      (`KismetSystemLibrary.PrintString` "Cast Failed"))))

(fn `UserConstructionScript`)