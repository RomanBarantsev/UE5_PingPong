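; BP_PingPongGameModeBase is a game mode Blueprint in the PingPong game that currently only prints debug messages for lifecycle events.
; It prints on BeginPlay, shows the end-play reason on EndPlay and names each new player on PostLogin.
; Tick prints the game's paused state every frame.
; The TestReady function and construction script are empty, so no match rules are implemented in these graphs.
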(event `self.ReceiveTick`
  (params (DeltaSeconds :type "Float (single-precision)"))
  (`KismetSystemLibrary.PrintString` (`KismetStringLibrary.Conv_BoolToString` (`GameplayStatics.IsGamePaused`)) true true (struct :`G` 0.66 :`B` 1.0 :`A` 1.0) 15.0))

(event `self.ReceiveBeginPlay`
  (`KismetSystemLibrary.PrintString` "BeginPlay" true true (struct :`G` 0.66 :`B` 1.0 :`A` 1.0) 15.0))

(event `self.ReceiveEndPlay`
  (params (EndPlayReason :type "EEndPlayReason Enum" :default "Destroyed"))
  (`KismetSystemLibrary.PrintString` (`|GetEnumeratorNameAsString` EndPlayReason) true true (struct :`G` 0.66 :`B` 1.0 :`A` 1.0) 15.0))

(event `self.K2_PostLogin`
  (params (NewPlayer :type "PlayerController Object Reference"))
  (`KismetSystemLibrary.PrintString` (`KismetSystemLibrary.GetDisplayName` NewPlayer) true true (struct :`G` 0.66 :`B` 1.0 :`A` 1.0) 15.0))

(fn `Test Ready`)

(fn `UserConstructionScript`)